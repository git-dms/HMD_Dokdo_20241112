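; BP_MasterButton is a VR world-space widget button that fills its WBP_Buttons widget with text and an index on BeginPlay.
; Tick smoothly turns its yaw to face the player.
; LobbyClear activates or deactivates the button by main-menu state, driving its scale with a forward or reversed timeline.
; A VR pawn entering its collision hides the button and, after a delay, toggles on the pawn's video button; leaving reverses this.
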(event `self.ReceiveBeginPlay`
  (`|ExecutionSequence`
    (:`then_0`
      (set `self.ButtonLocation` (`self.K2_GetActorLocation`)))
    (:`then_1`
      (bind _aswbp_buttons (cast `/Game/_Project/Blueprints/WBP_Buttons` (`WidgetComponent.GetUserWidgetObject` (`self.Button`))))
      (set `/Game/_Project/Blueprints/WBP_Buttons.Get Text` (`KismetTextLibrary.Conv_StringToText` (`self.Text Name`)) _aswbp_buttons)
      (set `/Game/_Project/Blueprints/WBP_Buttons.SetIndex` (`self.Index`) _aswbp_buttons))))

(event `self.ReceiveTick`
  (params (DeltaSeconds :type "Float (single-precision)"))
  (bind (_returnvalue_roll _returnvalue_pitch _returnvalue_yaw) (`KismetMathLibrary.BreakRotator` (`KismetMathLibrary.RInterpTo` (`self.K2_GetActorRotation`) (`KismetMathLibrary.FindLookAtRotation` (`self.K2_GetActorLocation`) (`self.K2_GetActorLocation` (`GameplayStatics.GetPlayerPawn` 0))) (`GameplayStatics.GetWorldDeltaSeconds`) 5.0)))
  (`self.K2_SetActorRotation` (`KismetMathLibrary.MakeRotator` 0.0 0.0 _returnvalue_yaw)))

(event `LobbyClear`
  (params (IsMainMenu :type Boolean :default false))
  (bind _button (`self.Button`))
  (if IsMainMenu
    (`ActorComponent.Deactivate` _button)
    (bind (_direction _alpha) (`Timeline|Timeline` :!via `Reverse` :!label _label)
      (:`Update`
        (`SceneComponent.SetRelativeScale3D` _button (`KismetMathLibrary.Conv_DoubleToVector` (* _alpha (`self.WidgetRelativeScaleOriginal`))))))
    (else
      (`ActorComponent.Activate` _button false)
      (goto _label))))

(event `self.Collision.OnComponentBeginOverlap`
  (params (OverlappedComponent :type "PrimitiveComponent Object Reference") (OtherActor :type "Actor Object Reference") (OtherComp :type "PrimitiveComponent Object Reference") (OtherBodyIndex :type Integer) (bFromSweep :type Boolean) (SweepResult :type "HitResult Structure (by ref)"))
  (bind _button (`self.Button`))
  (bind _asbp_vrpawn (cast `/Game/_Project/Blueprints/BP_VRPawn` OtherActor))
  (`SceneComponent.SetVisibility` _button false false)
  (`PrimitiveComponent.SetCollisionEnabled` _button "NoCollision")
  (`KismetSystemLibrary.Delay` 1.0)
  (`/Game/_Project/Blueprints/BP_VRPawn.ToggleVideoButton` _asbp_vrpawn true))

(event `self.Collision.OnComponentEndOverlap`
  (params (OverlappedComponent :type "PrimitiveComponent Object Reference") (OtherActor :type "Actor Object Reference") (OtherComp :type "PrimitiveComponent Object Reference") (OtherBodyIndex :type Integer))
  (bind _button (`self.Button`))
  (bind _asbp_vrpawn (cast `/Game/_Project/Blueprints/BP_VRPawn` OtherActor))
  (`SceneComponent.SetVisibility` _button true false)
  (`PrimitiveComponent.SetCollisionEnabled` _button "QueryAndPhysics")
  (`/Game/_Project/Blueprints/BP_VRPawn.ToggleVideoButton` _asbp_vrpawn false))

(fn `UserConstructionScript`)