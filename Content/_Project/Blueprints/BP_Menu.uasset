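; BP_Menu is a VR menu actor that shows a widget in front of the player and handles pointer clicks on it.
; On BeginPlay it enables input, attaches to the BP_VRPawn's CameraOrigin at a forward offset, and scales the widget in with a timeline.
; CloseMenu reverses that timeline, and the actor destroys itself when the reverse finishes.
; The right-hand shoot action presses and releases left mouse through its WidgetInteractionComponent.
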(event `self.ReceiveBeginPlay`
  (bind _relativescale3d_x (`KismetMathLibrary.BreakVector` (`SceneComponent.RelativeScale3D` (`self.Widget`))))
  (`|ExecutionSequence`
    (:`then_0`
      (`self.EnableInput` (`GameplayStatics.GetPlayerController` 0)))
    (:`then_1`
      (`self.K2_AttachToComponent` (`/Game/_Project/Blueprints/BP_VRPawn.CameraOrigin` (cast `/Game/_Project/Blueprints/BP_VRPawn` (`GameplayStatics.GetPlayerPawn` 0) :!pure true)) "None" "KeepRelative" "KeepRelative" "KeepRelative")
      (`self.K2_SetActorRelativeTransform` (`KismetMathLibrary.MakeTransform` (1000.0 0.0 0.0) (struct :`Yaw` 180.0)))
      (set `self.WidgetRelativeScaleOriginal` _relativescale3d_x) ; Set the original relative scale
      (bind (_direction _alpha) (`Timeline|Timeline` :!label _label)
        (:`Update`
          (`SceneComponent.SetRelativeScale3D` (`self.Widget`) (`KismetMathLibrary.Conv_DoubleToVector` (* _alpha (`self.WidgetRelativeScaleOriginal`)))))
        (:`Finished`
          (if (`|EnumEquality` _direction "Backward")
            (`self.K2_DestroyActor`)))))))

(event `CloseMenu`
  (goto _label :!via `Reverse`))

(event `EnhancedInput|/Game/_Project/Input/Actions/IA_Shoot_Right`
  (params (ActionValue :type Boolean) (ElapsedSeconds :type "Float (double-precision)") (TriggeredSeconds :type "Float (double-precision)") (InputAction :type "InputAction Object Reference" :default "/Game/_Project/Input/Actions/IA_Shoot_Right.IA_Shoot_Right"))
  (bind _widget_interaction_component (`self.Widget Interaction Component`))
  (:`Triggered`
    (`WidgetInteractionComponent.PressPointerKey` _widget_interaction_component "LeftMouseButton"))
  (:`Completed`
    (`WidgetInteractionComponent.ReleasePointerKey` _widget_interaction_component "LeftMouseButton")))

(fn `UserConstructionScript`)