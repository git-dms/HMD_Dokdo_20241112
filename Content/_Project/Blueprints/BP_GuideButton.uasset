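; BP_GuideButton is a guide button actor that shows a labeled WBP_Buttons widget and turns to face the player.
; BeginPlay sets the widget text from TextName, and Tick smoothly interpolates the actor's yaw toward the player pawn.
; LobbyClear toggles the widget by the IsMainMenu flag: true deactivates it and reverses a scale timeline, false activates it and plays the timeline forward.
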(event `self.ReceiveBeginPlay`
  (`|ExecutionSequence`
    (:`then_1`
      (bind _aswbp_buttons (cast `/Game/_Project/Blueprints/WBP_Buttons` (`WidgetComponent.GetUserWidgetObject` (`self.GuideButton`))))
      (set `/Game/_Project/Blueprints/WBP_Buttons.Get Text` (`KismetTextLibrary.Conv_StringToText` (`self.Text Name`)) _aswbp_buttons))))

(event `self.ReceiveTick`
  (params (DeltaSeconds :type "Float (single-precision)"))
  (bind (_returnvalue_roll _returnvalue_pitch _returnvalue_yaw) (`KismetMathLibrary.BreakRotator` (`KismetMathLibrary.RInterpTo` (`self.K2_GetActorRotation`) (`KismetMathLibrary.FindLookAtRotation` (`self.K2_GetActorLocation`) (`self.K2_GetActorLocation` (`GameplayStatics.GetPlayerPawn` 0))) (`GameplayStatics.GetWorldDeltaSeconds`) 5.0)))
  (`self.K2_SetActorRotation` (`KismetMathLibrary.MakeRotator` 0.0 0.0 _returnvalue_yaw)))

(event `LobbyClear`
  (params (IsMainMenu :type Boolean :default false))
  (bind _guidebutton (`self.GuideButton`))
  (if IsMainMenu
    (`ActorComponent.Deactivate` _guidebutton)
    (bind (_direction _alpha) (`Timeline|Timeline` :!via `Reverse` :!label _label)
      (:`Update`
        (`SceneComponent.SetRelativeScale3D` (`self.GuideButton`) (`KismetMathLibrary.Conv_DoubleToVector` (* _alpha (`self.WidgetRelativeScaleOriginal`))))))
    (else
      (`ActorComponent.Activate` _guidebutton false)
      (goto _label))))

(fn `UserConstructionScript`)