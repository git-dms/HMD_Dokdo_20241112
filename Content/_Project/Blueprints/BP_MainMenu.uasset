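; VR main menu actor that shows WBP_MainMenu in front of the player and fades it in and out.
; On BeginPlay it attaches to BP_VRPawn's CameraOrigin at a fixed offset and calls MainMenuControl.
; MainMenuControl toggles on IsMainMenuOn, using staggered timelines to fade title and buttons, and destroys the actor after fading out.
; The right-hand shoot input acts as a left mouse click through the WidgetInteractionComponent.
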(event `self.ReceiveBeginPlay`
  (`|ExecutionSequence`
    (:`then_0`
      (`self.EnableInput` (`GameplayStatics.GetPlayerController` 0)))
    (:`then_1`
      (`self.K2_AttachToComponent` (`/Game/_Project/Blueprints/BP_VRPawn.CameraOrigin` (cast `/Game/_Project/Blueprints/BP_VRPawn` (`GameplayStatics.GetPlayerPawn` 0) :!pure true)) "None" "KeepRelative" "KeepRelative" "KeepRelative")
      (`self.K2_SetActorRelativeTransform` (`KismetMathLibrary.MakeTransform` (1200.0 0.0 20.0)))
      (`self.Main Menu Control`))))

(event `self.ReceiveTick`
  (params (DeltaSeconds :type "Float (single-precision)")))

(event `Main Menu Control`
  (bind _aswbp_main_menu (cast `/Game/_Project/Blueprints/WBP_MainMenu` (`WidgetComponent.GetWidget` (`self.MainMenu`))))
  (if (`self.IsMainMenuOn`)
    (`|ExecutionSequence`
      (:`then_0`
        (set `self.IsMainMenuOn` false)
        (`|ExecutionSequence`
          (:`then_0`
            (`KismetSystemLibrary.Delay` 0.5)
            (bind (_direction _opacity) (`Timeline|Timeline_1` :!via `ReverseFromEnd`)
              (:`Update`
                (bind _titlebox (`/Game/_Project/Blueprints/WBP_MainMenu.TitleBox` _aswbp_main_menu))
                (`Widget.SetRenderOpacity` _titlebox _opacity))))
          (:`then_1`
            (`KismetSystemLibrary.Delay` 1.0)
            (bind (_direction_2 _opacity_2) (`Timeline|Timeline_2` :!via `ReverseFromEnd`)
              (:`Update`
                (bind _startbutton (`/Game/_Project/Blueprints/WBP_MainMenu.StartButton` _aswbp_main_menu))
                (`Widget.SetRenderOpacity` _startbutton _opacity_2)
                (`Widget.SetRenderOpacity` (`/Game/_Project/Blueprints/WBP_MainMenu.ExitButton` _aswbp_main_menu) _opacity_2)))))
        (`KismetSystemLibrary.Delay` (`self.FadingDuration`))
        (`self.K2_DestroyActor`)))
    (else
      (set `self.IsMainMenuOn` true)
      (`KismetSystemLibrary.Delay` (`self.FadingDuration`))
      (`|ExecutionSequence`
        (:`then_0`
          (bind (_direction_3 _opacity_3) (`Timeline|Timeline`)
            (:`Update`
              (`Widget.SetRenderOpacity` _titlebox _opacity_3))))
        (:`then_1`
          (`KismetSystemLibrary.Delay` 1.0)
          (bind (_direction_4 _opacity_4) (`Timeline|Timeline_0` :!via `PlayFromStart`)
            (:`Update`
              (`Widget.SetRenderOpacity` _startbutton _opacity_4)
              (`Widget.SetRenderOpacity` (`/Game/_Project/Blueprints/WBP_MainMenu.ExitButton` _aswbp_main_menu) _opacity_4))))))))

(event `EnhancedInput|/Game/_Project/Input/Actions/IA_Shoot_Right`
  (params (ActionValue :type Boolean) (ElapsedSeconds :type "Float (double-precision)") (TriggeredSeconds :type "Float (double-precision)") (InputAction :type "InputAction Object Reference" :default "/Game/_Project/Input/Actions/IA_Shoot_Right.IA_Shoot_Right"))
  (bind _widget_interaction_component (`self.Widget Interaction Component`))
  (:`Triggered`
    (`WidgetInteractionComponent.PressPointerKey` _widget_interaction_component "LeftMouseButton"))
  (:`Completed`
    (`WidgetInteractionComponent.ReleasePointerKey` _widget_interaction_component "LeftMouseButton")))

(fn `UserConstructionScript`)